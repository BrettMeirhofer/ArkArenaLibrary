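; BP_DividerWall is an arena divider wall actor that can be switched on and off.
; UpdateActivation sets the WallActivated variable, whose OnRep function shows or hides the static mesh and toggles its collision between query-and-physics and none.
; BeginPlay also calls that OnRep function after a short delay to apply the initial state.
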(event `self.ReceiveBeginPlay`
  (`KismetSystemLibrary.Delay` 0.2)
  (`self.OnRep_WallActivated`))

(event `UpdateActivation`
  (params (Toggle :type Boolean))
  (set `self.WallActivated` Toggle true))

(fn `OnRep_WallActivated`
  (bind _wallactivated (`self.WallActivated`))
  (bind _staticmesh1 (`self.StaticMesh1`))
  (`SceneComponent.SetVisibility` _staticmesh1 _wallactivated false)
  (if _wallactivated
    (`PrimitiveComponent.SetCollisionEnabled` _staticmesh1 "QueryAndPhysics")
    (else
      (`PrimitiveComponent.SetCollisionEnabled` _staticmesh1 "NoCollision"))))

(fn `UserConstructionScript`)