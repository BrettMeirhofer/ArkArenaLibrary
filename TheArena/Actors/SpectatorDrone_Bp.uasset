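; SpectatorDrone_Bp is a spectator drone actor for TheArena that appears to serve as a camera viewpoint with a fixed facing.
; Construction disables collision on its mesh, capsule and stasis component after running the parent script.
; Control rotation is overridden to follow the Arrow1 component's world rotation, with desired rotation reported as world space.
; BeginPlay only runs a short delay, and the owner controller view-target blend is disconnected.
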(event `self.ReceiveBeginPlay`
  (`KismetSystemLibrary.Delay` 0.2))

(fn `BPDesiredRotationIsLocalSpace`
  (returns (ReturnValue :type Boolean))
  (return false))

(fn `BPModifyControlRotation`
  (params (controlRotation :type "Object.Rotator Structure (by ref)"))
  (returns (outControlRotation :type "Object.Rotator Structure") (ReturnValue :type Boolean))
  (return (`SceneComponent.K2_GetComponentRotation` (`self.Arrow1`)) true))

(fn `UserConstructionScript`
  (`parent.UserConstructionScript`)
  (`PrimitiveComponent.SetCollisionEnabled` (`self.Mesh`) "NoCollision")
  (`PrimitiveComponent.SetCollisionEnabled` (`self.CapsuleComponent`) "NoCollision")
  (`PrimitiveComponent.SetCollisionEnabled` (`self.StasisComponent`) "NoCollision"))