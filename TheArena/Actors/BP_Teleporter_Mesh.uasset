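; Arena teleporter actor that sends a player to a random destination among actors sharing its custom tag.
; On the server, it strips the safe-zone buff and teleports through the XanjisFunctions helper's class default object.
; It also plays the teleport sound to controllers of red and blue arena team actors, skipping the traveler.
; The teleport check always passes, and arena status updates do nothing.
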(event EventArenaStatusUpdated
  (params (Status :type Byte :default 0)))

(fn ConstructionScript
  (|CallParentFunction))

(fn TeleportPlayer
  (params (InputPin :type Shooter%20Character%20Object%20Reference))
  (Networking|SwitchHasAuthority
    (:Authority
      (bind _asshootercharacter (Utilities|Casting|CastToShooterCharacter InputPin))
      (bind _returnvalue (Class|Actor|GetOwnerController _asshootercharacter))
      (bind _returnvalue_2 (Class|VictoryCore|GetClassDefaultObject "/Game/Mods/LibraryMod/HelperObject_XanjisFunctions.HelperObject_XanjisFunctions_C"))
      (bind _ashelperobject_xanjisfunctions_c (Utilities|Casting|CastToHelperObject_XanjisFunctions _returnvalue_2))
      (Default|DestroySpecificBuffs _ashelperobject_xanjisfunctions_c _asshootercharacter (Utilities|Array|MakeArray "/Game/Mods/LibraryMod/Buffs/Buff_SafeZone.Buff_SafeZone_C"))
      (bind _returnvalue_3 (Class|VictoryCore|GetCustomActorList (Class|Actor|GetWorld) (Variables|Default|GetCustomTag)))
      (LocalVariables|SetPointList (Variables|/Script/ShooterGame.CustomActorList|GetActorList _returnvalue_3))
      (bind _transform (Default|GetRandomDest _ashelperobject_xanjisfunctions_c (LocalVariables|GetPointList)))
      (Default|TeleportPlayer _ashelperobject_xanjisfunctions_c _asshootercharacter (Variables|Default|GetTeleportAudio) _transform)
      (for _array_element (Utilities|Array|MakeArray "RedTeamArena" "BlueTeamArena")
        (bind _returnvalue_4 (Class|VictoryCore|GetCustomActorList (Class|Actor|GetWorld) _array_element))
        (for _array_element_2 (Variables|/Script/ShooterGame.CustomActorList|GetActorList _returnvalue_4)
          (bind _returnvalue_5 (Class|Actor|GetOwnerController _array_element_2))
          (if (not (== _returnvalue _returnvalue_5))
            (bind _asshooterplayercontroller (Utilities|Casting|CastToShooterPlayerController _returnvalue_5))
            (Class|ShooterPlayerController|ClientPlayLocalSound _asshooterplayercontroller (Variables|Default|GetTeleportAudio) true)))))))

(fn CanTeleport
  (params (Char :type Shooter%20Character%20Object%20Reference))
  (return true))